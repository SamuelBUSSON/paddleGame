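; Networked physics ball for a paddle game, launched at a speed scaled by the game instance's Settings.
; On Tick, the authority passes location and velocity to Synchronize, then checks whether the ball passed the negative-X limit.
; An out-of-area ball explodes, resets to the origin, calls BallLeftArea and relaunches.
; Hits play sounds at the configured volume; paddle hits also spawn bounce particles and call HumanHit.
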(event Custom|OnBeginPlay
  (bind _assettings (Utilities|Casting|CastToSettings (Game|GetGameInstance)))
  (bind _output_get (Variables|Default|SetInitialSpeed (Variables|/Game/Settings.Settings_C|GetSpeed _assettings)))
  (Variables|Default|SetInitialVolume (Variables|/Game/Settings.Settings_C|GetSoundVolume _assettings))
  (Physics|SetPhysicsLinearVelocity (Variables|Default|GetStaticMesh) (* (Math|Vector|MakeVector 2e+03 2.25e+03 0.0) _output_get) false "None"))

(event Custom|Movement
  (bind _returnvalue (Transformation|GetActorLocation))
  (if (< (.X (Math|Vector|BreakVector _returnvalue)) -8.5e+02)
    (Audio|PlaySoundatLocation "/Game/Feedback/explosion.explosion" _returnvalue "0, 0, 0" (Variables|Default|GetInitialVolume) 1.0 0.0 0 0 0)
    (Effects|SpawnEmitteratLocation "/Game/Feedback/P_Explosion.P_Explosion" _returnvalue)
    (Transformation|SetActorLocation "0, 0,0.000000" false false)
    (Audio|PlaySoundatLocation "/Game/Feedback/bell.bell" "0, 0, 0" "0, 0, 0" (Variables|Default|GetInitialVolume) 1.0 0.0 0 0 0)
    (Default|CallBallLeftArea)
    (Physics|SetPhysicsLinearVelocity (Variables|Default|GetStaticMesh) (* (Math|Vector|MakeVector 2e+03 2.25e+03 0.0) (stale Custom|OnBeginPlay _output_get)) false "None")))

(event Custom|OnHit
  (params (Hit%20location :type Vector) (Other :type Actor%20Object%20Reference))
  (bind _initialvolume (Variables|Default|GetInitialVolume))
  (Utilities|Casting|CastToBP_Paddle Other
    (:then
      (Audio|PlaySoundatLocation "/Game/Feedback/ding.ding" Hit%20location "0, 0, 0" _initialvolume 1.0 0.0 0 0 0)
      (Effects|SpawnEmitteratLocation "/Game/Feedback/P_Bounce.P_Bounce" Hit%20location)
      (Default|CallHumanHit))
    (:CastFailed
      (Audio|PlaySoundatLocation "/Game/Feedback/pop.pop" Hit%20location "0, 0, 0" _initialvolume 1.0 0.0 0 0 0))))

(event Custom|Synchronize
  (params (Velocity :type Vector) (Location :type Vector))
  ;[1 1 1] Synchronize
  (Transformation|SetActorLocation Location false false)
  (Physics|SetPhysicsLinearVelocity (Variables|Default|GetStaticMesh) Velocity false "None"))

(event EventBeginPlay
  (CallFunction|OnBeginPlay))

(event EventTick
  (params (DeltaSeconds :type Float%20%28single-precision%29))
  ;[1 1 1] Synchronize
  (Networking|SwitchHasAuthority
    (:Authority
      (bind _returnvalue (Physics|GetPhysicsLinearVelocity (Variables|Default|GetStaticMesh) "None"))
      (CallFunction|Synchronize _returnvalue (Transformation|GetActorLocation))
      (CallFunction|Movement))))

(event Collision|EventHit
  (params (MyComp :type Primitive%20Component%20Object%20Reference) (Other :type Actor%20Object%20Reference) (OtherComp :type Primitive%20Component%20Object%20Reference) (bSelfMoved :type Boolean) (HitLocation :type Vector :default "0, 0, 0") (HitNormal :type Vector :default "0, 0, 0") (NormalImpulse :type Vector :default "0, 0, 0") (Hit :type Hit%20Result%20Structure%20%28by%20ref%29))
  (CallFunction|OnHit HitLocation Other))

(fn ConstructionScript)