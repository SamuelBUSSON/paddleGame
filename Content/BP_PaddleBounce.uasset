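; BP_PaddleBounce is the game mode for a paddle-and-ball game, tracking human and computer scores.
; It binds to BP_Ball events, scoring for the human on hits and for the computer when balls leave the area, and pushes totals to ScoreDisplay actors.
; An existing "all" save stores the high score, and three computer points load DemoMenu as a level instance.
; ChoosePlayerStart assigns P1- then P2-tagged starts using a player counter.
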(event Custom|IncrementComputer
  ;[1 1 1] Increment Computer Score
  (bind _result (Math|Integer|IncrementInt (Variables|Default|GetComputerScore))
    (:%20%20
      (bind _outactors (Actor|GetAllActorsOfClass "/Game/ScoreDisplay.ScoreDisplay_C"))
      (for _array_element _outactors
        (Default|SetComputerScore _array_element _result)
        (if (== _result 3)
          (Class|LevelStreamingKismet|LoadLevelInstancebySoftObjectPtr "/Game/Interface/DemoMenu.DemoMenu" "0, 0, 0" "0, 0, 0"))))))

(event Custom|IncrementHuman
  ;[1 1 1] Increment Human Score
  (bind _result (Math|Integer|IncrementInt (Variables|Default|GetHumanScore))
    (:%20%20
      (bind _outactors (Actor|GetAllActorsOfClass "/Game/ScoreDisplay.ScoreDisplay_C"))
      (for _array_element _outactors
        (Default|SetPlayerScore _array_element _result)
        (bind _returnvalue (SaveGame|DoesSaveGameExist "all"))
        (if _returnvalue
          (bind _returnvalue_2 (SaveGame|LoadGamefromSlot "all"))
          (bind _asbp_save_game (Utilities|Casting|CastToBP_SaveGame _returnvalue_2))
          (if (> _result (Variables|/Game/BP_SaveGame.BP_SaveGame_C|GetHighScore _asbp_save_game))
            (Variables|/Game/BP_SaveGame.BP_SaveGame_C|SetHighScore _asbp_save_game _result)
            (SaveGame|SaveGametoSlot _asbp_save_game "all")
            (bind _outactors_2 (Actor|GetAllActorsOfClass "/Game/ScoreDisplay.ScoreDisplay_C"))
            (for _array_element_2 _outactors_2
              (Default|SetHighScore _array_element_2 _result))))))))

(event EventBeginPlay
  (bind _outactors (Actor|GetAllActorsOfClass "/Game/BP_Ball.BP_Ball_C"))
  (for _array_element _outactors
    (EventDispatchers|BindEventtoBallLeftArea _array_element (delegate Custom|IncrementComputer))
    (EventDispatchers|BindEventtoHumanHit _array_element (delegate Custom|IncrementHuman))
    (bind _returnvalue (SaveGame|DoesSaveGameExist "all"))
    (if _returnvalue
      (bind _returnvalue_2 (SaveGame|LoadGamefromSlot "all"))
      (bind _asbp_save_game (Utilities|Casting|CastToBP_SaveGame _returnvalue_2))
      (bind _outactors_2 (Actor|GetAllActorsOfClass "/Game/ScoreDisplay.ScoreDisplay_C"))
      (for _array_element_2 _outactors_2
        (Default|SetHighScore _array_element_2 (Variables|/Game/BP_SaveGame.BP_SaveGame_C|GetHighScore _asbp_save_game))))))

(fn ConstructionScript)

(fn ChoosePlayerStart
  (params (Player :type Controller%20Object%20Reference))
  (if (== (Variables|Default|GetPlayerCount) 0)
    (bind _outactors (Actor|GetAllActorswithTag "P1"))
    (for _array_element _outactors
      (LocalVariables|SetPlayerStart _array_element)
      (Math|Integer|IncrementInt (Variables|Default|GetPlayerCount)
        (:%20%20
          (return (LocalVariables|GetPlayerStart)))))
    (else
      (bind _outactors_2 (Actor|GetAllActorswithTag "P2"))
      (for _array_element_2 _outactors_2
        (LocalVariables|SetPlayerStart _array_element_2)
        (Math|Integer|IncrementInt (Variables|Default|GetPlayerCount)
          (:%20%20
            (return (LocalVariables|GetPlayerStart))))))))